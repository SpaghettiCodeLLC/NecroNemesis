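; Gravetender NPC Blueprint that relays crystal collection and circle binding to its AI controller.
; On possession it casts the new controller to AIC_Gravetender and caches it.
; CollectCrystal and BindToCircle run their parent implementations first, then pass the collection result and IsBound state to that controller.
; GetNecromancerController is left empty.
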(event EventPossessed
  (params (NewController :type Controller%20Object%20Reference))
  (bind _asaic_gravetender (Utilities|Casting|CastToAIC_Gravetender NewController))
  (Variables|Default|SetGravetenderController _asaic_gravetender))

(fn ConstructionScript)

(fn GetNecromancerController)

(fn CollectCrystal
  (bind _hascrystal (|CallParentFunction))
  (Default|CollectCrystal (Variables|Default|GetGravetenderController) _hascrystal))

(fn BindtoCircle
  (|CallParentFunction)
  (Default|BindtoCircle (Variables|Default|GetGravetenderController) (Variables|Default|GetbIsBound)))