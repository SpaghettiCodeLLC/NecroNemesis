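; BP_Minion is a minion NPC with an affiliation tag, a child-actor weapon and a Bones/Souls/Gold cost, controlled by AIC_Minion.
; Damage goes to HealthComponent, then a Combat.Status.Damaged gameplay tag blocks further hits until a timer clears it after DamageInterval.
; A health-change dispatcher destroys the actor on death; the health bar widget code is disconnected.
; Getters expose health, tagging and weapon, and Tick prints a warning when any cost is negative.
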(event Custom|HandleHealthUpdate_Event
  (params (Percentage :type Float%20%28double-precision%29) (Dead? :type Boolean))
  (if Dead?
    (Actor|DestroyActor)))

(event Custom|ResetDamagedStatus
  (bind _taggingcomponent (Variables|Default|GetTaggingComponent))
  (Utilities|IsValid _taggingcomponent
    (:Is%20Valid
      (Default|RemoveGameplayTag _taggingcomponent "(TagName=\"Combat.Status.Damaged\")"))))

(event EventBeginPlay
  (Default|AddGameplayTag (Variables|Default|GetTaggingComponent) (Variables|Minion|Info|GetAffiliation))
  (EventDispatchers|BindEventtoDispatchHealthChangeUpdate (Variables|Default|GetHealthComponent) (EventDispatchers|CreateEvent :!event Custom|HandleHealthUpdate_Event))
  (bind _asbp_weapon (Utilities|Casting|CastToBP_Weapon (Variables|/Script/Engine.ChildActorComponent|GetChildActor (Variables|Default|GetBP_Weapon)))
    (:then
      (Variables|Default|SetWeapon _asbp_weapon))
    (:CastFailed
      (Development|PrintString "No weapon on zombie"))))

(event EventPossessed
  (params (NewController :type Controller%20Object%20Reference))
  (bind _asaic_minion (Utilities|Casting|CastToAIC_Minion NewController))
  (Variables|AI|SetMinionController _asaic_minion))

(event EventTick
  (params (DeltaSeconds :type Float%20%28single-precision%29))
  (bind _minioncost (Variables|Minion|Info|GetMinionCost))
  (if (not (Math|Boolean|ANDBoolean (>= (.bones _minioncost) 0) (>= (.souls _minioncost) 0) (>= (.gold _minioncost) 0)))
    (Development|PrintString (Utilities|String|Append (Utilities|GetDisplayName self) " doesn't have a cost set"))))

(event EventTakeDamage
  (params (DamageDetails :type F%20Damage%20Info%20Structure))
  (bind _returnvalue (Default|HasOneTag (Variables|Default|GetTaggingComponent) "(TagName=\"Combat.Status.Damaged\")" true))
  (if (not _returnvalue)
    (Default|TakeDamage (Variables|Default|GetHealthComponent) (.basedamage DamageDetails))
    (Utilities|IsValid (Variables|Default|GetTaggingComponent)
      (:Is%20Valid
        (Default|AddGameplayTag (Variables|Default|GetTaggingComponent) "(TagName=\"Combat.Status.Damaged\")")
        (bind _returnvalue_2 (Utilities|Time|SetTimerbyEvent (delegate Custom|ResetDamagedStatus) (Variables|Default|GetDamageInterval)))
        (Variables|Default|SetDamageStatusResetTimerHandle _returnvalue_2)))))

(event EventEndPlay
  (params (EndPlayReason :type EEndPlayReason%20Enum :default "Destroyed"))
  (EventDispatchers|UnbindEventfromDispatchHealthChangeUpdate (Variables|Default|GetHealthComponent) (EventDispatchers|CreateEvent :!event Custom|HandleHealthUpdate_Event))
  (Utilities|Time|ClearandInvalidateTimerbyHandle (Variables|Default|GetDamageStatusResetTimerHandle)))

(fn ConstructionScript
  (Variables|Minion|Info|SetHalfHeight (Variables|/Script/Engine.CapsuleComponent|GetCapsuleHalfHeight (Variables|Default|GetCapsule))))

(fn SetAffiliationID
  (params (AffiliationID :type Name))
  (bind _output_get (Variables|Minion|Info|SetAffiliationID AffiliationID))
  (Utilities|Array|Add (Variables|Actor|GetTags) _output_get))

(fn GetDamageInfo)

(fn GetGameplayTagContainer
  (return ""))

(fn GetHealthComponent
  (return (Variables|Default|GetHealthComponent)))

(fn GetTaggingComponent
  (return (Variables|Default|GetTaggingComponent)))

(fn GetWeapon
  (return (Variables|Default|GetWeapon)))

(fn HasGameplayTag?
  (params (Tag :type Gameplay%20Tag%20Structure) (ExactMatch :type Boolean))
  (bind _returnvalue (Default|HasOneTag (Variables|Default|GetTaggingComponent) Tag ExactMatch))
  (return _returnvalue))

(fn RemoveGameplayTagfromTarget
  (return false))