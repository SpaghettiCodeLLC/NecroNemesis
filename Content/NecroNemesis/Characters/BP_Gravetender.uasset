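; Gravetender character that carries bones and souls and auto-deposits them into the Ossuary when its capsule overlaps a summoning circle.
; Construction maps AffiliationID to an actor tag and gameplay tag; BeginPlay registers it with the LaneGenerator and wires up its child-actor weapon.
; Weapon attack events toggle an Attacking status tag on the TaggingComponent.
; Helpers detect attached summoning crystals and flag binding to a circle; several getters are stubs.
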(event OnComponentBeginOverlap(CapsuleComponent)
  (params (OverlappedComponent :type Primitive%20Component%20Object%20Reference) (OtherActor :type Actor%20Object%20Reference) (OtherComp :type Primitive%20Component%20Object%20Reference) (OtherBodyIndex :type Integer) (bFromSweep :type Boolean) (SweepResult :type Hit%20Result%20Structure%20%28by%20ref%29))
  ;[1 1 1] Autodeposit to Ossuary
  (if (Actor|ActorHasTag OtherActor "SCircle")
    (bind _asbp_summoning_circle (Utilities|Casting|CastToBP_SummoningCircle OtherActor))
    (Default|DeposittoOssuary _asbp_summoning_circle (Variables|PlayerInfo|GetResourceComponent))))

(event EventBeginPlay
  (CallFunction|SetupWeapon)
  (bind _returnvalue (Actor|GetActorOfClass "/Game/NecroNemesis/Core/Interactables/LaneGenerator.LaneGenerator_C"))
  (Variables|/Game/NecroNemesis/Core/Interactables/LaneGenerator.LaneGenerator_C|SetTenderReference _returnvalue self))

(event EventTick
  (params (DeltaSeconds :type Float%20%28single-precision%29)))

(fn ConstructionScript
  (bind _gameplaytags (Variables|PlayerInfo|GetGameplayTags))
  (bind _affiliationid (Variables|PlayerInfo|GetAffiliationID))
  (Utilities|Array|Add (Variables|Actor|GetTags) _affiliationid)
  (switch name _affiliationid
    (:Unum
      ;[1 1 1] Initial Impl.
      ; TODO: Set on Spawn
      (GameplayTags|AddGameplayTag _gameplaytags (GameplayTags|MakeLiteralGameplayTag "(TagName=\"Affiliation.Unum\")") :!class /Script/GameplayTags.BlueprintGameplayTagLibrary))
    (:Duo
      (GameplayTags|AddGameplayTag _gameplaytags (GameplayTags|MakeLiteralGameplayTag "(TagName=\"Affiliation.Duo\")") :!class /Script/GameplayTags.BlueprintGameplayTagLibrary))
    (:Tres
      (GameplayTags|AddGameplayTag _gameplaytags (GameplayTags|MakeLiteralGameplayTag "(TagName=\"Affiliation.Tres\")") :!class /Script/GameplayTags.BlueprintGameplayTagLibrary))
    (:Quatuor
      (GameplayTags|AddGameplayTag _gameplaytags (GameplayTags|MakeLiteralGameplayTag "(TagName=\"Affiliation.Quattuor\")") :!class /Script/GameplayTags.BlueprintGameplayTagLibrary))
    (:Quintum
      (GameplayTags|AddGameplayTag _gameplaytags (GameplayTags|MakeLiteralGameplayTag "(TagName=\"Affiliation.Quintum\")") :!class /Script/GameplayTags.BlueprintGameplayTagLibrary))))

(fn AddtoCharnelSatchel
  (params (ResourceType :type EResourceType%20Enum :default "NewEnumerator0") (Amount :type Integer))
  (bind _resourcecomponent (Variables|PlayerInfo|GetResourceComponent))
  (switch Utilities|FlowControl|Switch|SwitchonEResourceType ResourceType
    (:NewEnumerator0
      (Default|AddBones _resourcecomponent Amount))
    (:NewEnumerator1
      (Default|AddSouls _resourcecomponent Amount))))

(fn CollectCrystal
  (bind _filteredarray (Utilities|Array|FilterArray (Actor|GetAttachedActors true false) "/Game/NecroNemesis/Core/Pickups/BP_Resource_SummoningCrystal.BP_Resource_SummoningCrystal_C"))
  (if (> (Utilities|Array|Length _filteredarray) 0)
    (Variables|Default|SetbHasCrystal true)
    (else
      (Variables|Default|SetbHasCrystal false)))
  (return (Variables|Default|GetbHasCrystal)))

(fn BindtoCircle
  (Variables|Default|SetbHasCrystal false)
  (Variables|PlayerInfo|SetbIsBound true)
  (return))

(fn SetupWeapon
  (Utilities|FlowControl|Sequence
    (:then_0
      ;[1 1 1] Get Weapon Reference.
      (bind _asbp_weapon (Utilities|Casting|CastToBP_Weapon (Variables|/Script/Engine.ChildActorComponent|GetChildActor (Variables|Default|GetWeapon)))
        (:then
          (Variables|Default|SetEquippedWeapon _asbp_weapon))
        (:CastFailed
          (Development|PrintString (Utilities|String|Append "WeaponError: " (Utilities|GetDisplayName self) " does not have a Weapon reference. Something Went Wrong (TM)")))))
    (:then_1
      ;[1 1 1] Set the current Tender to the Weapon
      (Variables|/Game/NecroNemesis/Core/Characters/Components/Weapons/BP_Weapon.BP_Weapon_C|SetTender (Variables|Default|GetEquippedWeapon) self))
    (:then_2
      ;[1 1 1] Set Weapon's damage details
      (Variables|/Game/NecroNemesis/Core/Characters/Components/Weapons/BP_Weapon.BP_Weapon_C|SetDamageDetails (Variables|Default|GetEquippedWeapon) (Utilities|Struct|MakeFDamageInfo self (.weapon (Variables|/Game/NecroNemesis/Core/Characters/Components/Weapons/BP_Weapon.BP_Weapon_C|GetDamageDetails (Variables|Default|GetEquippedWeapon))) (.basedamage (Variables|/Game/NecroNemesis/Core/Characters/Components/Weapons/BP_Weapon.BP_Weapon_C|GetDamageDetails (Variables|Default|GetEquippedWeapon))) (.damagetype (Variables|/Game/NecroNemesis/Core/Characters/Components/Weapons/BP_Weapon.BP_Weapon_C|GetDamageDetails (Variables|Default|GetEquippedWeapon))) (.aggrodelta (Variables|/Game/NecroNemesis/Core/Characters/Components/Weapons/BP_Weapon.BP_Weapon_C|GetDamageDetails (Variables|Default|GetEquippedWeapon))))))
    (:then_3
      (EventDispatchers|BindEventtoHandleStartAttack (Variables|Default|GetEquippedWeapon) (EventDispatchers|CreateEvent :!event HandleAttackStart))
      (EventDispatchers|BindEventtoHandleEndAttack (Variables|Default|GetEquippedWeapon) (EventDispatchers|CreateEvent :!event HandleAttackEnd)))))

(fn HandleAttackStart
  (Default|AddGameplayTag (Variables|Default|GetTaggingComponent) "(TagName=\"Status.Tender.Combat.Attacking\")"))

(fn HandleAttackEnd
  (Default|RemoveGameplayTag (Variables|Default|GetTaggingComponent) "(TagName=\"Status.Tender.Combat.Attacking\")"))

(fn GetDamageInfo)

(fn GetGameplayTagContainer
  (return (Variables|PlayerInfo|GetGameplayTags)))

(fn GetTaggingComponent
  (return 0))

(fn GetWeapon
  (return (Variables|Default|GetEquippedWeapon)))

(fn RemoveGameplayTagfromTarget
  (return false))