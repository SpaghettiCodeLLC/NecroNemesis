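; BP_Weapon is a melee weapon that detects hits during an attack and deals damage.
; StartAttack line-traces between the mesh's start and end sockets and sends TakeDamageMessage to a hit actor implementing BPI_Damageable, ignoring the wielding Tender.
; A second debug-drawn trace links the previous and current start-socket positions, but its result is unused.
; EndAttack clears the Tender's attacking gameplay tag and resets the stored position flag.
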(event Custom|StartAttack
  (bind _array (Utilities|Array|MakeArray "ObjectTypeQuery6" "ObjectTypeQuery7" "ObjectTypeQuery10"))
  (bind _weaponmesh (Variables|Default|GetWeaponMesh))
  (bind _tender (Variables|Default|GetTender))
  (bind _returnvalue (Transformation|GetSocketLocation _weaponmesh "start"))
  (bind _array_2 (Utilities|Array|MakeArray _tender))
  (if (Variables|Default|GetbLastLocationSet)
    (Collision|LineTraceForObjects (Variables|Default|GetLastLocation) _returnvalue _array false _array_2 "ForDuration" true "(R=1.000000,G=0.693893,B=0.000000,A=1.000000)" "(R=0.000000,G=0.149850,B=1.000000,A=1.000000)"))
  (bind _outhit (Collision|LineTraceForObjects _returnvalue (Transformation|GetSocketLocation _weaponmesh "end") _array false _array_2 "ForDuration"))
  (Variables|Default|SetLastLocation _returnvalue)
  (Variables|Default|SetbLastLocationSet true)
  (if (not (not (Utilities|DoesObjectImplementInterface (.hitactor _outhit) "/Game/NecroNemesis/Core/Characters/Components/BPI_Damageable.BPI_Damageable_C")))
    (Class|BPIDamageable|TakeDamage(Message) (.hitactor _outhit) (Variables|Default|GetDamageDetails))))

(event Custom|EndAttack
  (GameplayTags|RemoveGameplayTag (Variables|/Game/NecroNemesis/Characters/BP_Gravetender.BP_Gravetender_C|GetGameplayTags (Variables|Default|GetTender)) "(TagName=\"Status.Tender.Combat.Attacking\")" :!class /Script/GameplayTags.BlueprintGameplayTagLibrary)
  (Variables|Default|SetbLastLocationSet false))

(fn ConstructionScript)