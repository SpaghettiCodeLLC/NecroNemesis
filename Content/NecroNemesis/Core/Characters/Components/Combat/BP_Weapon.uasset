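; BP_Weapon is a melee weapon actor that traces its swing and damages whatever it hits.
; On construction it collects mesh sockets named with "atk_sock_" as trace points.
; StartAttack runs a looping timer that line-traces from each socket's previous position to its current one, gathers unique BPI_Damageable hits per tick and applies base damage through their health components.
; EndAttack stops the timer and clears the Tender's Attacking tag.
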(event Custom|StartAttack
  (bind _returnvalue (Utilities|Time|SetTimerbyEvent (delegate Custom|BeginTrace) (Variables|Trace|GetWeaponTraceCheckInterval) true))
  (Variables|Trace|SetTraceTimerHandle _returnvalue)
  (Default|CallDispatchStartAttack))

(event Custom|BeginTrace
  (Utilities|Array|Clear (Variables|Default|GetHitDamageables))
  (if (Variables|Default|GetbLastLocationSet)
    (for (_array_element _array_index) (Variables|Default|GetLastLocation)
      (bind _outhits (Collision|MultiLineTraceByChannel _array_element (Transformation|GetSocketLocation (Variables|Default|GetWeaponMesh) (Utilities|Array|Get(acopy) (Variables|Default|GetSocketNames) _array_index)) "TraceTypeQuery1" false (Utilities|Array|MakeArray (Variables|Default|GetTender)) "ForDuration"))
      (for _array_element_2 _outhits
        (if (Utilities|DoesObjectImplementInterface (.hitactor _array_element_2) "/Game/NecroNemesis/Core/Characters/Components/Combat/BPI_Damageable.BPI_Damageable_C")
          (bind _asbpi_damageable (Utilities|Casting|CastToBPI_Damageable (.hitactor _array_element_2)))
          (Utilities|Array|AddUnique (Variables|Default|GetHitDamageables) _asbpi_damageable)))))
  (for (_array_element_3 _array_index_2) (Variables|Default|GetSocketNames)
    (Utilities|Array|SetArrayElem (Variables|Default|GetLastLocation) _array_index_2 (Transformation|GetSocketLocation (Variables|Default|GetWeaponMesh) _array_element_3)))
  (Variables|Default|SetbLastLocationSet true)
  (for _array_element_4 (Variables|Default|GetHitDamageables)
    (bind _healthcomponent (Default|GetHealthComponent _array_element_4))
    (Default|TakeDamage _healthcomponent (.basedamage (Variables|Combat|GetDamageDetails)))))

(event Custom|EndAttack
  (bind _tender (Variables|Default|GetTender))
  (Utilities|Time|ClearandInvalidateTimerbyHandle (Variables|Trace|GetTraceTimerHandle))
  (Utilities|IsValid _tender
    (:Is%20Valid
      (Default|RemoveGameplayTag (Variables|/Game/NecroNemesis/Characters/BP_Gravetender.BP_Gravetender_C|GetTaggingComponent _tender) "(TagName=\"Status.Tender.Combat.Attacking\")"))
    (:Is%20Not%20Valid
      _))
  (Variables|Default|SetbLastLocationSet false)
  (Default|CallDispatchEndAttack))

(event EventBeginPlay
  (Default|AddGameplayTag (Variables|Default|GetTaggingComponent) "(TagName=\"Combat.Damage.Bludgeon\")")
  (Variables|Combat|SetDamageDetails (Utilities|Struct|MakeFDamageInfo (.instigator (Variables|Combat|GetDamageDetails)) self (.basedamage (Variables|Combat|GetDamageDetails)) (.damagetype (Variables|Combat|GetDamageDetails)) (.aggrodelta (Variables|Combat|GetDamageDetails)))))

(fn ConstructionScript
  (Construction|ConstructSocketNameArray)
  (Utilities|Array|Resize (Variables|Default|GetLastLocation) (Utilities|Array|Length (Variables|Default|GetSocketNames))))

(fn ConstructSocketNameArray
  (for _array_element (Transformation|GetAllSocketNames (Variables|Default|GetWeaponMesh))
    (if (Utilities|String|Contains (Utilities|String|ToString(Name) _array_element) "atk_sock_")
      (Utilities|Array|AddUnique (Variables|Default|GetSocketNames) _array_element)))
  (if (Utilities|Array|IsEmpty (Variables|Default|GetSocketNames))
    (Development|PrintString "Fatal Error: Weapon does not have any atk_sock_ Socket set up on Mesh. ")
    (else
      (return))))