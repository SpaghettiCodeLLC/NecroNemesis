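; BP_Factory is an actor-spawning factory that places a requested class on the surface below a given transform.
; RequestActorSpawn traces downward on Visibility and spawns slightly above the hit, with the requester as Owner and Instigator, ignoring its Key.
; FindRequestedActor looks up classes in the ClassTypes map by key.
; An older map-based spawn path with failure reporting and destroyed-event binding is disconnected, leaving the destruction logger unbound here.
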(fn RequestActorSpawn
  (params (Key :type Name) (Requester :type Pawn%20Object%20Reference) (SpawnLocation :type Transform) (Class :type Actor%20Class%20Reference))
  (bind (_location _rotation _scale) (Math|Transform|BreakTransform SpawnLocation))
  (bind _outhit (Collision|LineTraceByChannel _location (- _location "0.000000,0.000000,1000.000000") "TraceTypeQuery1" false 0 "ForDuration"))
  (bind _returnvalue (Game|SpawnActorfromClass Class (Math|Transform|MakeTransform (+ (.location _outhit) "0.000000,0.000000,120.000000") _rotation _scale) "Undefined" "MultiplyWithRoot" Requester Requester))
  (return _returnvalue))

(fn HandleActorDestroyedEvent
  (params (DestroyedActor :type Actor%20Object%20Reference))
  (Development|PrintString (Utilities|String|Append (Utilities|GetDisplayName DestroyedActor) " is Destroyed from the Factory.")))

(fn FindRequestedActor
  (params (ActorKey :type Name))
  (bind _classtypes (Variables|Default|GetClassTypes))
  (bind (_value _returnvalue) (Utilities|Map|Find _classtypes ActorKey))
  (return _value _returnvalue))