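; Minion factory that spawns minions for Gravetenders and looks up their cost from class defaults by spawn key.
; Spawns go through RequestActorSpawn, either by key with a height offset or by class at an indexed lane transform.
; Each minion's AI controller receives its affiliation and target summoning circle.
; Key-based spawns bind a destroyed handler, which calls the parent, prints debug text and reports the minion's death.
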(event Custom|RequestMinionSpawn
  (params (SpawnKey :type Name) (BoundGravetender :type BP%20Gravetender%20Object%20Reference) (SpawnTransform :type Transform) (AffiliationID :type Name) (TargetSummoningCircle :type BP%20Summoning%20Circle%20Object%20Reference))
  (bind (_location _rotation _scale) (Math|Transform|BreakTransform SpawnTransform))
  (bind _spawnedactor (CallFunction|RequestActorSpawn SpawnKey BoundGravetender (Math|Transform|MakeTransform (+ _location "0.000000,0.000000,80.000000") _rotation _scale)))
  (Game|BindEventtoOnDestroyed _spawnedactor (delegate EventHandleActorDestroyedEvent))
  (CallFunction|InitializeSpawnedMinion _spawnedactor AffiliationID TargetSummoningCircle))

(event EventHandleActorDestroyedEvent
  (params (DestroyedActor :type Actor%20Object%20Reference))
  (|CallParentFunction DestroyedActor)
  (Development|PrintString (Utilities|String|Append "And now in the Minion Factory    " (Utilities|GetDisplayName DestroyedActor) "    " (Utilities|String|ToString(Vector) (Transformation|GetActorLocation DestroyedActor))))
  (bind _asbp_minion (Utilities|Casting|CastToBP_Minion DestroyedActor))
  (Default|CallHandleMinionDeath _asbp_minion))

(fn InitializeSpawnedMinion
  (params (Minion :type Actor%20Object%20Reference) (AffiliationID :type Name) (TargetCircle :type BP%20Summoning%20Circle%20Object%20Reference))
  (bind _asaic_minion (Utilities|Casting|CastToAIC_Minion (AI|GetAIController Minion)))
  (Default|InitializeSpawn _asaic_minion AffiliationID TargetCircle))

(fn GetMinionCost
  (params (SpawnKey :type Name))
  (bind _classtypes (Variables|Default|GetClassTypes))
  (bind (_value _returnvalue) (Utilities|Map|Find _classtypes SpawnKey))
  (if _returnvalue
    (bind _asbp_minion (Utilities|Casting|CastToBP_MinionClass _value)
      (:then
        (return (.MinionCost (Utilities|GetClassDefaults _asbp_minion))))
      (:CastFailed
        _)))
  (return ""))

(fn SpawnLaneMinion
  (params (Tender :type BP%20Gravetender%20Object%20Reference) (Minion :type BP%20Minion%20Class%20Reference) (SpawnTransforms :type Array%20of%20Transforms) (Idx :type Integer) (TargetCircle :type BP%20Summoning%20Circle%20Object%20Reference))
  (bind _miniontospawn (CallFunction|ConstructMinionSpawnRequest Minion))
  (bind _spawnedactor (CallFunction|RequestActorSpawn "None" Tender (Utilities|Array|Get(acopy) SpawnTransforms Idx) _miniontospawn))
  (bind _asbp_minion (Utilities|Casting|CastToBP_Minion _spawnedactor))
  (Default|InitializeSpawn (Variables|/Game/NecroNemesis/Characters/NPC/Minion/BP_Minion.BP_Minion_C|GetMinionController _asbp_minion) (Variables|/Game/NecroNemesis/Characters/BP_Gravetender.BP_Gravetender_C|GetAffiliationID Tender) TargetCircle)
  (return))

(fn ConstructMinionSpawnRequest
  (params (Minion :type BP%20Minion%20Class%20Reference))
  (if (Utilities|IsValidClass Minion)
    (LocalVariables|SetTempCurrentMinionClass Minion))
  (return (LocalVariables|GetTempCurrentMinionClass)))