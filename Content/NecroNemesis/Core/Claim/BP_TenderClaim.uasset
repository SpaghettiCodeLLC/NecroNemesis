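; BP_TenderClaim is a damageable claim actor that shows a health bar and destroys itself when its health runs out.
; TakeDamage passes base damage to its HealthComponent, whose update dispatcher drives the health bar widget and the destroy check.
; The dispatcher is bound on BeginPlay and unbound on EndPlay.
; Its gameplay tag, damage info and weapon getter functions are empty stubs that return default values.
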(event Custom|HandleHealthUpdate_Event
  (params (HealthPercentage :type Float%20%28double-precision%29))
  (Default|UpdateHealthBar (Variables|Default|GetHealthBarWidget) HealthPercentage)
  (if (<= HealthPercentage 0.0)
    (Actor|DestroyActor)))

(event EventBeginPlay
  (bind _aswbp_health_bar (Utilities|Casting|CastToWBP_HealthBar (UserInterface|GetUserWidgetObject (Variables|Default|GetHealthBar))))
  (Variables|Default|SetHealthBarWidget _aswbp_health_bar)
  (EventDispatchers|BindEventtoDispatchHealthUpdate (Variables|Default|GetHealthComponent) (EventDispatchers|CreateEvent :!event Custom|HandleHealthUpdate_Event)))

(event Collision|EventActorBeginOverlap
  (params (OtherActor :type Actor%20Object%20Reference)))

(event EventTick
  (params (DeltaSeconds :type Float%20%28single-precision%29)))

(event EventTakeDamage
  (params (DamageDetails :type F%20Damage%20Info%20Structure))
  (Default|TakeDamage (Variables|Default|GetHealthComponent) (.basedamage DamageDetails)))

(event EventEndPlay
  (params (EndPlayReason :type EEndPlayReason%20Enum :default "Destroyed"))
  (EventDispatchers|UnbindEventfromDispatchHealthUpdate (Variables|Default|GetHealthComponent) (EventDispatchers|CreateEvent :!event Custom|HandleHealthUpdate_Event)))

(fn ConstructionScript)

(fn GetDamageInfo
  (return ""))

(fn GetGameplayTagContainer
  (return ""))

(fn GetTaggingComponent
  (return 0))

(fn GetWeapon
  (return 0))

(fn HasGameplayTag?
  (params (Tag :type Gameplay%20Tag%20Structure) (ExactMatch :type Boolean))
  (return false))

(fn RemoveGameplayTagfromTarget
  (return false))