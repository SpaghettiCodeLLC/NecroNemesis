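; Game mode for NecroNemesis that sets up summoning circles and local player Gravetenders, and brokers minion and resource spawning.
; On BeginPlay it maps circles by affiliation tag, shares them with GameState and possesses one Gravetender per player; NPC spawning is switched off.
; Circle, grave and minion-death events route to minion and resource factories.
; Minion requests check and charge the Ossuary, but failed checks only print without halting the spawn sequence.
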(event Custom|HandleMinionDeath_Event
  (params (Minion :type BP%20Minion%20Object%20Reference))
  (CallFunction|HandleMinionDeath Minion))

(event Custom|HandleRequestMinionSpawn_Event
  (params (SpawnKey :type Name) (BoundGravetender :type BP%20Gravetender%20Object%20Reference) (SpawnLocation :type Transform) (AffiliationID :type Name) (TargetSummoningCircle :type BP%20Summoning%20Circle%20Object%20Reference) (Ossuary :type BP%20Ossuary%20Object%20Reference))
  (CallFunction|HandleSummoningCircleSpawnRequest SpawnKey BoundGravetender SpawnLocation AffiliationID TargetSummoningCircle Ossuary))

(event Custom|HandleRequestEmptyGraveContents_Event
  (params (GraveType :type EGraveType%20Enum :default "NewEnumerator2") (SpawnTransform :type Transform))
  (CallFunction|HandleEmptyGraveContents GraveType SpawnTransform))

(event EventBeginPlay
  (Utilities|FlowControl|Sequence
    (:then_0
      (Construction|SetupGameInstanceReference))
    (:then_1
      (Construction|SetupGameStateReference))
    (:then_2
      (bind _successful (Construction|ConstructSummoningCircleMap))
      (if (not _successful)
        (Development|PrintString "Critical Failure: Unable to find Summoning Circles. 
This... shouldn't happen. ERR: 7070707" true true "(R=1.000000,G=0.000000,B=0.000000,A=1.000000)" 5.0)))
    (:then_3
      (Construction|ConstructTargetingArrays))
    (:then_4
      (Construction|SpawnGravetenders false) ; SpawnNPC: allows much easier solo debugging without NPC Gravetenders spawning. Please take care not to ship with it unchecked....
    )
    (:then_5
      (bind _values (Utilities|Map|Values (Variables|GameInfo|GamePieces|GetSummoningCircles)))
      (for _array_element _values
        (EventDispatchers|AssignHandleRequestMinionSpawn _array_element (delegate Custom|HandleRequestMinionSpawn_Event))
        (for _array_element_2 (Variables|/Game/NecroNemesis/Core/Interactables/BP_SummoningCircle.BP_SummoningCircle_C|GetGraveyard _array_element)
          (EventDispatchers|BindEventtoRequestGraveContents _array_element_2 (delegate Custom|HandleRequestEmptyGraveContents_Event)))))
    (:then_6
      (EventDispatchers|BindEventtoHandleMinionDeath (Variables|Default|GetBP_Factory_Minion) (delegate Custom|HandleMinionDeath_Event)))))

(fn ConstructionScript)

(fn SetupGameInstanceReference
  (bind _asbp_necro_nemesis_game_instance (Utilities|Casting|CastToBP_NecroNemesisGameInstance (Game|GetGameInstance)))
  (bind _output_get (Variables|Core|SetInstance _asbp_necro_nemesis_game_instance))
  (Development|PrintString (Utilities|String|Append "Game Instance Successfully Setup." "   |   Total Number of PCs: " (Utilities|String|ToString(Integer) (Variables|/Game/NecroNemesis/Core/GameModes/BP_NecroNemesisGameInstance.BP_NecroNemesisGameInstance_C|GetNumberOfPlayers _output_get)) "   |   Remaining Gravetenders will become AI Controlled: " (Utilities|String|ToString(Integer) (- 5 (Variables|/Game/NecroNemesis/Core/GameModes/BP_NecroNemesisGameInstance.BP_NecroNemesisGameInstance_C|GetNumberOfPlayers _output_get))))))

(fn SetupGameStateReference
  (bind _asbp_necro_nemesis_game_state (Utilities|Casting|CastToBP_NecroNemesisGameState (Game|GetGameState)))
  (Variables|Core|SetState _asbp_necro_nemesis_game_state)
  (return))

(fn ConstructSummoningCircleMap
  (Utilities|Map|Clear (Variables|GameInfo|GamePieces|GetSummoningCircles))
  (bind _outactors (Actor|GetAllActorsOfClass "/Game/NecroNemesis/Core/Interactables/BP_SummoningCircle.BP_SummoningCircle_C"))
  (for _array_element _outactors
    (Utilities|Map|Add (Variables|GameInfo|GamePieces|GetSummoningCircles) (Utilities|Array|Get(acopy) (Variables|/Script/Engine.Actor|GetTags _array_element) 1) _array_element))
  (return (> (Utilities|Map|Length (Variables|GameInfo|GamePieces|GetSummoningCircles)) 0)))

(fn SpawnGravetenders
  (params (SpawnNPC :type Boolean))
  (for _index (range 0 (- (Variables|/Game/NecroNemesis/Core/GameModes/BP_NecroNemesisGameInstance.BP_NecroNemesisGameInstance_C|GetNumberOfPlayers (Variables|Core|GetInstance)) 1)) ; SpawnPC
    (Construction|CreatePCGravetender _index))
  (if SpawnNPC
    (Construction|CreateNPCGravetenders)))

(fn CreatePCGravetender
  (params (Idx :type Integer))
  (bind _output_get (LocalVariables|SetIndex Idx))
  (Utilities|IsValid (Game|GetPlayerController _output_get)
    (:Is%20Valid
      (bind _asbp_gravetender_controller_pc (Utilities|Casting|CastToCtrl_Gravetender (Game|GetPlayerController _output_get))
        (:then
          (LocalVariables|SetCurrentController _asbp_gravetender_controller_pc)
          (switch int (LocalVariables|GetIndex) :!label _label
            (:0
              (LocalVariables|SetAffiliationID "Unum"))
            (:1
              (LocalVariables|SetAffiliationID "Duo"))
            (:2
              (LocalVariables|SetAffiliationID "Tres"))
            (:3
              (LocalVariables|SetAffiliationID "Quattuor"))
            (:4
              (LocalVariables|SetAffiliationID "Quintum")))
          (if (.ReturnValue (Utilities|Map|Find (Variables|GameInfo|GamePieces|GetSummoningCircles) (LocalVariables|GetAffiliationID)))
            (bind _playerstart (Default|GetPlayerStart (.Value (Utilities|Map|Find (Variables|GameInfo|GamePieces|GetSummoningCircles) (LocalVariables|GetAffiliationID)))))
            (bind _returnvalue (Game|SpawnActorfromClass "/Game/NecroNemesis/Characters/PC/BP_Gravetender_PC.BP_Gravetender_PC_C" _playerstart "Undefined" "MultiplyWithRoot" 0 (.Value (Utilities|Map|Find (Variables|GameInfo|GamePieces|GetSummoningCircles) (LocalVariables|GetAffiliationID))) (LocalVariables|GetAffiliationID) 0))
            (Utilities|Map|Add (Variables|GameInfo|GamePieces|GetGravetenders) (LocalVariables|GetAffiliationID) _returnvalue)
            (Utilities|IsValid (Pawn|GetControlledPawn (LocalVariables|GetCurrentController))
              (:Is%20Valid
                (Actor|DestroyActor (Pawn|GetControlledPawn (LocalVariables|GetCurrentController))))
              (:Is%20Not%20Valid
                _))
            (Pawn|Possess (LocalVariables|GetCurrentController) _returnvalue)))
        (:CastFailed
          (Development|PrintString "GameMode: Failed to Cast to GravetenderController. " :!label _label_2))))
    (:Is%20Not%20Valid
      (bind _returnvalue_2 (Class|GameplayStatics|CreatePlayer -1))
      (bind _asbp_gravetender_controller_pc_2 (Utilities|Casting|CastToCtrl_Gravetender _returnvalue_2)
        (:then
          (LocalVariables|SetCurrentController _asbp_gravetender_controller_pc_2)
          (goto _label))
        (:CastFailed
          (goto _label_2))))))

(fn CreateNPCGravetenders
  (for _index (range 0 (Utilities|Operators|Subtract (Variables|GameInfo|GetMaxPlayers) (Variables|/Game/NecroNemesis/Core/GameModes/BP_NecroNemesisGameInstance.BP_NecroNemesisGameInstance_C|GetNumberOfPlayers (Variables|Core|GetInstance)) 1)) ; SpawnNPC
    (switch int (+ _index (Variables|/Game/NecroNemesis/Core/GameModes/BP_NecroNemesisGameInstance.BP_NecroNemesisGameInstance_C|GetNumberOfPlayers (Variables|Core|GetInstance)))
      (:0
        (Development|PrintString "Error: Should not be here GAMEMODE"))
      (:1
        (LocalVariables|SetAffiliationID "Duo")
        (if (.ReturnValue (Utilities|Map|Find (Variables|GameInfo|GamePieces|GetSummoningCircles) (LocalVariables|GetAffiliationID))) :!label _label
          (bind _playerstart (Default|GetPlayerStart (.Value (Utilities|Map|Find (Variables|GameInfo|GamePieces|GetSummoningCircles) (LocalVariables|GetAffiliationID)))))
          (Game|SpawnActorfromClass "/Game/NecroNemesis/Characters/NPC/Gravetender/BP_Gravetender_NPC.BP_Gravetender_NPC_C" _playerstart "Undefined" "MultiplyWithRoot" 0 (.Value (Utilities|Map|Find (Variables|GameInfo|GamePieces|GetSummoningCircles) (LocalVariables|GetAffiliationID))) (LocalVariables|GetAffiliationID) 0)))
      (:2
        (LocalVariables|SetAffiliationID "Tres")
        (goto _label))
      (:3
        (LocalVariables|SetAffiliationID "Quattuor")
        (goto _label))
      (:4
        (LocalVariables|SetAffiliationID "Quintum")
        (goto _label)))))

(fn ConstructTargetingArrays
  (bind _output_get (Variables|/Game/NecroNemesis/Core/GameModes/BP_NecroNemesisGameState.BP_NecroNemesisGameState_C|SetSummoningCircles (Variables|Core|GetState) (Variables|GameInfo|GamePieces|GetSummoningCircles)))
  (bind _values (Utilities|Map|Values _output_get))
  (for _array_element _values
    (Default|InitializeCircle _array_element)))

(fn ConstructPitMap
  (bind _outactors (Actor|GetAllActorsOfClass "/Game/NecroNemesis/Core/Interactables/BP_Pit.BP_Pit_C"))
  (Variables|Default|SetPitArray _outactors))

(fn ValidateMinionCostRequirements
  (params (ActorClass :type Actor%20Class%20Reference) (Ossuary :type BP%20Ossuary%20Object%20Reference))
  (bind _asbp_minion (Utilities|Casting|CastToBP_MinionClass ActorClass))
  (return (and (>= (Variables|/Game/NecroNemesis/Core/Interactables/BP_Ossuary.BP_Ossuary_C|GetTotal%20Bones Ossuary) (.Bones (Utilities|Struct|BreakFMinionCost (.MinionCost (Utilities|GetClassDefaults _asbp_minion))))) (>= (Variables|/Game/NecroNemesis/Core/Interactables/BP_Ossuary.BP_Ossuary_C|GetTotal%20Souls Ossuary) (.Souls (Utilities|Struct|BreakFMinionCost (.MinionCost (Utilities|GetClassDefaults _asbp_minion)))))) (.MinionCost (Utilities|GetClassDefaults _asbp_minion))))

(fn HandleSummoningCircleSpawnRequest
  (params (SpawnKey :type Name) (BoundGravetender :type BP%20Gravetender%20Object%20Reference) (SpawnTransform :type Transform) (AffiliationID :type Name) (TargetSummoningCircle :type BP%20Summoning%20Circle%20Object%20Reference) (Ossuary :type BP%20Ossuary%20Object%20Reference))
  (LocalVariables|SetTempKey SpawnKey)
  (Utilities|FlowControl|Sequence
    (:then_0
      ;[1 1 1] Find Requested Spawn
      (bind (_actorclass _bisfound) (Default|FindRequestedActor (Variables|Default|GetBP_Factory_Minion) (LocalVariables|GetTempKey)))
      (if _bisfound
        (LocalVariables|SetTempClass _actorclass)
        (else
          (Development|PrintString "Could not find requested Spawn in the Factory Map."))))
    (:then_1
      ;[1 1 1] Validate Cost of Spawn
      (bind (_bcostrequirementsmet _spawn_cost) (CallFunction|ValidateMinionCostRequirements (LocalVariables|GetTempClass) Ossuary))
      (if _bcostrequirementsmet
        (LocalVariables|SetRequestedCost _spawn_cost)
        (else
          (Development|PrintString "Not enough Resources in the Ossuary"))))
    (:then_2
      ;[1 1 1] Charge Ossuary
      (bind _successful (Default|Charge Ossuary (LocalVariables|GetRequestedCost)))
      (if (not _successful)
        (Development|PrintString "Something very strange occured. The Ossuary was brought to a negative value after a Minion Spawn request. ")))
    (:then_3
      ;[1 1 1] Call for Spawn
      (Default|RequestMinionSpawn (Variables|Default|GetBP_Factory_Minion) (LocalVariables|GetTempKey) BoundGravetender SpawnTransform AffiliationID TargetSummoningCircle))))

(fn HandleMinionDeath
  (params (Minion :type BP%20Minion%20Object%20Reference))
  (Default|RequestMinionDeathResourceSpawn (Variables|Default|GetBP_Factory_Resource) (Variables|/Game/NecroNemesis/Characters/NPC/Minion/BP_Minion.BP_Minion_C|GetMinionCost Minion) (Transformation|GetActorTransform Minion)))

(fn HandleEmptyGraveContents
  (params (GraveType :type EGraveType%20Enum :default "NewEnumerator2") (SpawnTransform :type Transform))
  (switch Utilities|FlowControl|Switch|SwitchonEGraveType GraveType
    (:NewEnumerator3
      (CallFunction|HandleSpawnRequest SpawnTransform))
    (:NewEnumerator2
      (Default|RequestGraveResourceContents (Variables|Default|GetBP_Factory_Resource) GraveType SpawnTransform :!label _label))
    (:NewEnumerator4
      (goto _label))))

(fn HandleResourceRequest
  (params (SpawnTransform :type Transform))
  (Default|RequestGraveResourceContents (Variables|Default|GetBP_Factory_Resource) "NewEnumerator2" SpawnTransform))

(fn HandleSpawnRequest
  (params (SpawnTransform :type Transform))
  ;[1 1 1] Neutral Spawn. World Event, essentially
  (Default|RequestMinionSpawn (Variables|Default|GetBP_Factory_Minion) "Zombie_001" 0 SpawnTransform "None"))

(fn HandleCrystalRequest
  (params (SpawnTransform :type Transform)))