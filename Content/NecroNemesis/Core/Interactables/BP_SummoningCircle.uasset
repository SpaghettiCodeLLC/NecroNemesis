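; Team summoning circle that a crystal-carrying Gravetender binds to, starting timed zombie spawns from its graveyard.
; InitializeCircle maps rival circles, aims and sizes Niagara tethers toward them, randomizes grave types and picks a crystal grave.
; Each spawn request targets a random rival circle, while overlapping toggles the bound PC's summoning input and targeting UI.
; It emits periodic AI noise, and depleted health destroys it, its Gravetender and all actors sharing its AffiliationID tag.
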(event OnComponentBeginOverlap(Sphere)
  (params (OverlappedComponent :type Primitive%20Component%20Object%20Reference) (OtherActor :type Actor%20Object%20Reference) (OtherComp :type Primitive%20Component%20Object%20Reference) (OtherBodyIndex :type Integer) (bFromSweep :type Boolean) (SweepResult :type Hit%20Result%20Structure%20%28by%20ref%29))
  ;[1 1 1] Activate Summoning UI (and handle initial binding)
  (bind _gravetender (Utilities|GravetenderCheck OtherActor)
    (:Successful
      (Utilities|BoundCheck :!label _label
        (:Bound
          (Utilities|PCCheck _gravetender
            (:True
              (PC|HandleInputMappingforPCNecromancer) ; Add summoning input
              (PC|SetupSummoningHUD))))
        (:Unbound
          (CircleActivation|HandleCircleActivation _gravetender)
          (if (Variables|CircleInfo|GetbIsBound)
            (CircleActivation|ToggleTethers -1)
            ;;[1 1 1] MinionSpawning. TODO: Change to toggle
            (Utilities|Time|SetTimerbyEvent (delegate Custom|SpawnArmy) (Variables|Summoning|GetSpawnInterval) true 1.25 0.25)
            (CircleActivation|HandleNecromancerBinding _gravetender)
            (goto _label)))))))

(event OnComponentEndOverlap(Sphere)
  (params (OverlappedComponent :type Primitive%20Component%20Object%20Reference) (OtherActor :type Actor%20Object%20Reference) (OtherComp :type Primitive%20Component%20Object%20Reference) (OtherBodyIndex :type Integer))
  ;[1 1 1] Deactivate SummoningUI
  (bind _gravetender (Utilities|GravetenderCheck OtherActor)
    (:Successful
      (Utilities|BoundCheck
        (:Bound
          (Utilities|PCCheck _gravetender
            (:True
              (PC|HandleInputMappingforPCNecromancer) ; Remove Summoning Input
              (Widget|RemovefromParent (Variables|UI|GetSummoningUI)))))))))

(event Custom|SpawnArmy
  ;[1 1 1] Activate Summoning UI (and handle initial binding)
  ;;[1 1 1] MinionSpawning. TODO: Change to toggle
  (Spawning|RequestSpawn "Zombie_001"))

(event Custom|InitializeCircle
  (Construction|GetGameState)
  (Construction|ConstructTargetingArray)
  (Construction|ConstructGraveyard)
  (CallFunction|RandomizeGraveContents)
  (Construction|ChooseCrystalGrave))

(event Custom|DingDONG
  (Class|AISenseHearing|ReportNoiseEvent (Transformation|GetWorldLocation (Variables|Default|GetSM_crystal_001)) 1.0 self 0.0 "DingDONG"))

(event EventBeginPlay
  (bind _aswbp_summoning_circle_health_bar (Utilities|Casting|CastToWBP_SummoningCircle_HealthBar (UserInterface|GetUserWidgetObject (Variables|UI|GetWGT_HealthBar))))
  (Variables|/Game/NecroNemesis/UI/WBP_SummoningCircle_HealthBar.WBP_SummoningCircle_HealthBar_C|SetOwningCircle _aswbp_summoning_circle_health_bar self)
  (Utilities|Time|SetTimerbyEvent (delegate Custom|DingDONG) 3e+01 true))

(event EventTakeDamage
  (params (DamageDetails :type F%20Damage%20Info%20Structure))
  (bind _output_get (Variables|/Game/NecroNemesis/Core/Characters/Components/Combat/HealthComponent.HealthComponent_C|SetCurrentHealth (Variables|CircleInfo|GetBP_HealthComponent) (- (Variables|/Game/NecroNemesis/Core/Characters/Components/Combat/HealthComponent.HealthComponent_C|GetCurrentHealth (Variables|CircleInfo|GetBP_HealthComponent)) (.basedamage DamageDetails))))
  (if (not (>= _output_get 0.0))
    (bind _outactors (Actor|GetAllActorswithTag (Variables|CircleInfo|GetAffiliationID)))
    (Utilities|Array|RemoveItem _outactors self)
    (Utilities|Array|RemoveItem _outactors (Variables|Summoning|GetBoundGravetender))
    (bind _arrayelement (Utilities|Array|ReverseforEachLoop _outactors)
      (:LoopBody
        (Actor|DestroyActor _arrayelement))
      (:Completed
        (Actor|DestroyActor (Variables|Summoning|GetBoundGravetender))
        (Development|PrintString (Utilities|String|Append (Utilities|GetDisplayName (Variables|/Script/Engine.Actor|GetInstigator (.instigator DamageDetails))) " drew last blood on " (Utilities|GetDisplayName self)))
        (Actor|DestroyActor)))))

(fn ConstructionScript
  (Variables|CircleInfo|SetAffiliationID (Utilities|Array|Get(acopy) (Variables|Actor|GetTags) 1)))

(fn RequestSpawn
  (params (SpawnKey :type Name))
  (bind _spawntransform (Spawning|GetSpawnLocation))
  (Default|CallHandleRequestMinionSpawn SpawnKey (Variables|Summoning|GetBoundGravetender) _spawntransform (Variables|CircleInfo|GetAffiliationID) (.OutItem (Utilities|Array|Random (Variables|Targeting|GetTargetCircleArray))) (Variables|Default|GetBP_Ossuary)))

(fn HandleInputMappingforPCNecromancer
  (bind _asctrl_gravetender (Utilities|Casting|CastToCtrl_Gravetender (Pawn|GetController (Variables|Summoning|GetBoundGravetender))))
  (Default|HandleInputMappingContext _asctrl_gravetender (Variables|Summoning|GetSummonInputContext)))

(fn HandleNecromancerBinding
  (params (Gravetender :type BP%20Gravetender%20Object%20Reference))
  (LocalVariables|SetRef Gravetender)
  (Utilities|IsValid (Variables|Summoning|GetBoundGravetender)
    (:Is%20Valid
      _)
    (:Is%20Not%20Valid
      (Variables|Summoning|SetBoundGravetender (LocalVariables|GetRef))))
  (return))

(fn GetPlayerStart
  (return (Transformation|GetWorldTransform (Variables|CircleInfo|GetPlayerSpawnPoint))))

(fn ConstructGraveyard
  (bind _outactors (Actor|GetAllActorsOfClasswithTag "/Game/NecroNemesis/Core/Interactables/BP_Grave.BP_Grave_C" (Variables|CircleInfo|GetAffiliationID)))
  (Variables|Summoning|SetGraveyard _outactors))

(fn ChooseCrystalGrave
  (bind _output_get (LocalVariables|SetCrystalGrave (.OutItem (Utilities|Array|Random (Variables|Summoning|GetGraveyard)))))
  (Utilities|IsValid _output_get
    (:Is%20Valid
      (Default|SetGraveType (LocalVariables|GetCrystalGrave) "NewEnumerator4")
      (Rendering|Material|SetMaterial (Variables|/Game/NecroNemesis/Core/Interactables/BP_Grave.BP_Grave_C|GetGraveMesh (LocalVariables|GetCrystalGrave)) 0 "/Engine/MapTemplates/Materials/BasicAsset01.BasicAsset01"))
    (:Is%20Not%20Valid
      (Development|PrintString (Utilities|String|Append "Graves are not set up around " (Utilities|String|ToString(Name) (Variables|CircleInfo|GetAffiliationID)))))))

(fn ConstructTargetingArray
  (CallFunction|ConstructTargetMap)
  (CallFunction|SetTetherRotation)
  (CircleActivation|SetTetherLengths))

(fn GetGameState
  (bind _asbp_necro_nemesis_game_state (Utilities|Casting|CastToBP_NecroNemesisGameState (Game|GetGameState))
    (:then
      (Variables|Components|SetGameState _asbp_necro_nemesis_game_state))
    (:CastFailed
      (Development|PrintString "CastFailed: Unable to cast to GameState in SummoningCircle"))))

(fn RegisterIncomingTargetAcquisition
  (params (IncomingCircle :type BP%20Summoning%20Circle%20Object%20Reference)))

(fn ToggleTethers
  (params (TetherIdx :type Integer))
  (bind _tether_1 (Variables|Default|GetTether_1))
  (switch int TetherIdx
    (:Default
      (Components|Activation|Activate _tether_1 false))
    (:0
      (Components|Activation|ToggleActive (Variables|Default|GetTether)))
    (:1
      (Components|Activation|ToggleActive _tether_1))
    (:2
      (Components|Activation|ToggleActive (Variables|Default|GetTether_2)))
    (:3
      (Components|Activation|ToggleActive (Variables|Default|GetTether_3)))))

(fn HandleCircleActivation
  (params (GT :type BP%20Gravetender%20Object%20Reference))
  (if (Variables|/Game/NecroNemesis/Characters/BP_Gravetender.BP_Gravetender_C|GetbHasCrystal GT) ; TODO: Take crystal from Gravetender and set in circle
    (bind _filteredarray (Utilities|Array|FilterArray (Actor|GetAttachedActors GT true false) "/Game/NecroNemesis/Core/Pickups/BP_Resource_SummoningCrystal.BP_Resource_SummoningCrystal_C"))
    (if (> (Utilities|Array|Length _filteredarray) 0)
      (Actor|DestroyActor (Utilities|Array|Get(acopy) _filteredarray))
      (Development|SetHiddeninGame (Variables|Default|GetSM_crystal_001) false true)
      (Default|BindtoCircle GT)
      (Variables|CircleInfo|SetbIsBound true)
      (return))
    (else
      (Development|PrintString "Go Find the Crystal") ; TODO: A popup, perhaps, that says this?
    )))

(fn SetupSummoningHUD
  (bind _asbp_gravetender_pc (Utilities|Casting|CastToBP_Gravetender_PC (Variables|Summoning|GetBoundGravetender)))
  (bind _returnvalue (UserInterface|CreateWidget "/Game/NecroNemesis/UI/WBP_SummoningCircle_Targeting.WBP_SummoningCircle_Targeting_C" (Variables|/Game/NecroNemesis/Characters/PC/BP_Gravetender_PC.BP_Gravetender_PC_C|GetGravetenderController _asbp_gravetender_pc) self))
  (bind _output_get (Variables|UI|SetSummoningUI _returnvalue))
  (UserInterface|Viewport|AddtoViewport _output_get 0)
  (Variables|/Script/Engine.PlayerController|SetbShowMouseCursor (Variables|/Game/NecroNemesis/Characters/PC/BP_Gravetender_PC.BP_Gravetender_PC_C|GetGravetenderController _asbp_gravetender_pc) true))

(fn SetTetherLengths
  (bind _values (Utilities|Map|Values (Variables|Targeting|GetTargetCircles)))
  (for (_array_element _array_index) _values
    (LocalVariables|SetForwardVelocity (/ (Math|Vector|Distance(Vector) (Transformation|GetSocketLocation (Variables|Default|GetSummoningCircleMesh) "crystal") (Transformation|GetSocketLocation (Variables|BP_SummoningCircle_C|GetSummoningCircleMesh (.targetcircle _array_element)) "crystal")) 2.0))
    (switch int _array_index
      (:0
        (Effects|Components|ParticleSystem|SetFloatParameter (Variables|Default|GetTether) "ForwardVelocity" (LocalVariables|GetForwardVelocity)) ; Dynamic beam extension. If the distance between Circles change, this should update just fine
      )
      (:1
        (Effects|Components|ParticleSystem|SetFloatParameter (Variables|Default|GetTether_1) "ForwardVelocity" (LocalVariables|GetForwardVelocity)) ; Dynamic beam extension. If the distance between Circles change, this should update just fine
      )
      (:2
        (Effects|Components|ParticleSystem|SetFloatParameter (Variables|Default|GetTether_2) "ForwardVelocity" (LocalVariables|GetForwardVelocity)) ; Dynamic beam extension. If the distance between Circles change, this should update just fine
      )
      (:3
        (Effects|Components|ParticleSystem|SetFloatParameter (Variables|Default|GetTether_3) "ForwardVelocity" (LocalVariables|GetForwardVelocity)) ; Dynamic beam extension. If the distance between Circles change, this should update just fine
      ))))

(fn GetSpawnLocation
  (bind _graveyard (Variables|Summoning|GetGraveyard))
  (if (Utilities|Array|IsNotEmpty _graveyard)
    (bind _output_get (LocalVariables|SetRandomGrave (.OutItem (Utilities|Array|Random _graveyard))))
    (return (Math|Transform|MakeTransform (+ (.location (Transformation|GetActorTransform _output_get)) "0.000000,0.000000,60.000000") (.rotation (Transformation|GetActorTransform _output_get)) "1.000000,1.000000,1.000000"))
    (else
      (Development|PrintString "empty graveyard?"))))

(fn SetTetherRotation
  (bind _values (Utilities|Map|Values (Variables|Targeting|GetTargetCircles)))
  (for (_array_element _array_index) _values
    (LocalVariables|SetNewYaw (.yaw (Math|Rotator|FindLookatRotation (Transformation|GetActorLocation self) (Transformation|GetActorLocation (.targetcircle _array_element)))))
    (switch int _array_index
      (:0
        (LocalVariables|SetTempTether (Variables|Default|GetTether)))
      (:1
        (LocalVariables|SetTempTether (Variables|Default|GetTether_1)))
      (:2
        (LocalVariables|SetTempTether (Variables|Default|GetTether_2)))
      (:3
        (LocalVariables|SetTempTether (Variables|Default|GetTether_3))))
    (Transformation|SetWorldRotation (LocalVariables|GetTempTether) (Math|Rotator|MakeRotator 0.0 0.0 (LocalVariables|GetNewYaw)) false false)))

(fn ConstructTargetMap
  (Utilities|Map|Clear (Variables|Targeting|GetTargetCircles))
  (Utilities|Array|Clear (Variables|Targeting|GetTargetCircleArray))
  (bind _values (Utilities|Map|Values (Variables|/Game/NecroNemesis/Core/GameModes/BP_NecroNemesisGameState.BP_NecroNemesisGameState_C|GetSummoningCircles (Variables|Components|GetGameState))))
  (for _array_element _values
    (if (not (== _array_element self))
      (LocalVariables|SetTempCircle _array_element)
      (Utilities|Map|Add (Variables|Targeting|GetTargetCircles) (Utilities|Array|Get(acopy) (Variables|/Script/Engine.Actor|GetTags (LocalVariables|GetTempCircle)) 1) (Utilities|Struct|MakeFCircleTargetingStruct (LocalVariables|GetTempCircle) true false))
      (Utilities|Array|Add (Variables|Targeting|GetTargetCircleArray) (LocalVariables|GetTempCircle)))))

(fn RandomizeGraveContents
  (bind _graveyard (Variables|Summoning|GetGraveyard))
  (LocalVariables|SetNeutralSpawnTotal (/ (Utilities|Array|Length _graveyard) 3))
  (Utilities|Array|Shuffle _graveyard)
  (for (_array_element _array_index) _graveyard
    (if (< _array_index (LocalVariables|GetNeutralSpawnTotal))
      (Variables|/Game/NecroNemesis/Core/Interactables/BP_Grave.BP_Grave_C|SetGraveType _array_element "NewEnumerator3")
      (Rendering|Material|SetMaterial (Variables|/Game/NecroNemesis/Core/Interactables/BP_Grave.BP_Grave_C|GetGraveMesh _array_element) 0 "/Engine/EngineDebugMaterials/VertexColorViewMode_GreenOnly.VertexColorViewMode_GreenOnly")
      (else
        (Variables|/Game/NecroNemesis/Core/Interactables/BP_Grave.BP_Grave_C|SetGraveType _array_element "NewEnumerator2")))))

(fn GetDamageInfo
  (return ""))

(fn GetHealthComponent
  (return 0))

(fn GetWeapon
  (return 0))