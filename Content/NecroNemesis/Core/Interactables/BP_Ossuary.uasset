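; BP_Ossuary is the resource bank in NecroNemesis, holding total bones, souls and gold.
; It seeds these totals from default values on BeginPlay, and Deposit adds bones and souls from a CharnelSatchel.
; Charge subtracts a MinionCost without checking first, since the GameMode validates requests, and returns whether all totals stay non-negative.
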(event EventBeginPlay
  (Setup|SetDefaultOssuaryValues))

(event EventTick
  (params (DeltaSeconds :type Float%20%28single-precision%29)))

(fn Deposit
  (params (CharnelSatchel :type BP%20Charnel%20Satchel%20Object%20Reference))
  (Variables|Resources|SetTotal%20Bones (+ (Variables|Resources|GetTotal%20Bones) (Variables|/Game/NecroNemesis/Core/Characters/Components/BP_CharnelSatchel.BP_CharnelSatchel_C|GetTotalBones CharnelSatchel)))
  (Variables|Resources|SetTotal%20Souls (+ (Variables|Resources|GetTotal%20Souls) (Variables|/Game/NecroNemesis/Core/Characters/Components/BP_CharnelSatchel.BP_CharnelSatchel_C|GetTotalSouls CharnelSatchel)))
  (return))

(fn SetDefaultOssuaryValues
  (Variables|Resources|SetTotal%20Bones (Variables|Setup|GetDefaultBones))
  (Variables|Resources|SetTotal%20Souls (Variables|Setup|GetDefaultSouls))
  (Variables|Resources|SetTotalGold (Variables|Setup|GetDefaultGold)))

(fn Charge
  (params (MinionCost :type F%20Minion%20Cost%20Structure))
  ;[1 1 1] Charge
  ; Charges the Ossuary the passed MinionCost struct.
  ; This charge is validated in the GameMode, ensuring that the Ossuary has enough Resources for the Request.
  ;
  ; Returns true as long as the Resources don't fall into the negative range (This shouldn't happen, although I have suspicions that it may happen in the case that the Request charges down to zero at the same time an auto Minion Spawn occurs.)
  (Utilities|FlowControl|Sequence
    (:then_0
      (Variables|Resources|SetTotal%20Bones (- (Variables|Resources|GetTotal%20Bones) (.bones MinionCost))))
    (:then_1
      (Variables|Resources|SetTotal%20Souls (- (Variables|Resources|GetTotal%20Souls) (.souls MinionCost))))
    (:then_2
      (Variables|Resources|SetTotalGold (- (Variables|Resources|GetTotalGold) (.gold MinionCost))))
    (:then_3
      ;;[1 1 1] Ensure
      (return (Math|Boolean|ANDBoolean (>= (Variables|Resources|GetTotal%20Bones) 0) (>= (Variables|Resources|GetTotal%20Souls) 0) (>= (Variables|Resources|GetTotalGold) 0))))))