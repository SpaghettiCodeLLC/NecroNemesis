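; BP_Grave is a diggable grave that requests its contents by grave type once digging completes, then recharges on a timer.
; A trigger box toggles the dig progress widget for non-NPC actors, turning it toward the player's camera.
; Dig events fill the bar; Tick shows the remaining recharge time until the grave is ready.
; Crystal graves register a hearing stimulus source and periodically report noise for AI perception.
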(event OnComponentBeginOverlap(Box)
  (params (OverlappedComponent :type Primitive%20Component%20Object%20Reference) (OtherActor :type Actor%20Object%20Reference) (OtherComp :type Primitive%20Component%20Object%20Reference) (OtherBodyIndex :type Integer) (bFromSweep :type Boolean) (SweepResult :type Hit%20Result%20Structure%20%28by%20ref%29))
  (if (not (Actor|ActorHasTag OtherActor "NPC"))
    (Development|SetHiddeninGame (Variables|Default|GetDigProgress) false false)
    (bind _as__tender_pc (Utilities|Casting|CastTo__Tender_PC OtherActor))
    (Variables|Default|SetInteractingCamera (Variables|/Game/NecroNemesis/Characters/PC/__Tender_PC.__Tender_PC_C|GetFollowCamera _as__tender_pc))))

(event OnComponentEndOverlap(Box)
  (params (OverlappedComponent :type Primitive%20Component%20Object%20Reference) (OtherActor :type Actor%20Object%20Reference) (OtherComp :type Primitive%20Component%20Object%20Reference) (OtherBodyIndex :type Integer))
  (if (not (Actor|ActorHasTag OtherActor "NPC"))
    (Development|SetHiddeninGame (Variables|Default|GetDigProgress) true false)
    (Variables|Default|SetInteractingCamera 0)))

(event Custom|OnGraveDug
  (params (DigTime :type Float%20%28double-precision%29) (Gravetender :type Tender%20Object%20Reference))
  (bind _output_get (Variables|/Game/NecroNemesis/UI/WBP_InteractionProgressBar.WBP_InteractionProgressBar_C|SetProgress (Variables|Default|GetGraveDigProgress) (/ DigTime (Variables|/Game/NecroNemesis/Characters/__Tender.__Tender_C|GetDigTime Gravetender))))
  (if (>= _output_get 1.0)
    (Development|SetHiddeninGame (Variables|Default|GetDigProgress) true false)
    (if (Variables|Default|GetbResourcesAvailable)
      (Default|CallRequestGraveContents (Variables|Default|GetGraveType) (Transformation|GetActorTransform))
      (Variables|Default|SetbResourcesAvailable false)
      (bind _returnvalue (Utilities|Time|SetTimerbyEvent (delegate Custom|OnGraveRefreshed) (Variables|Default|GetRechargeTime)))
      (Variables|Default|SetRechargeTimer _returnvalue))))

(event Custom|OnGraveRefreshed
  (Variables|Default|SetbResourcesAvailable true)
  (Rendering|Components|TextRender|SetText (Variables|Default|GetTimerText) (Utilities|Text|MakeLiteralText "Grave Ready!")))

(event EventBeginPlay
  (Variables|Default|SetbResourcesAvailable true)
  (bind _aswbp_grave_dig_progress (Utilities|Casting|CastToWBP_InteractionProgressBar (UserInterface|GetUserWidgetObject (Variables|Default|GetDigProgress))))
  (Variables|Default|SetGraveDigProgress _aswbp_grave_dig_progress))

(event EventTick
  (params (DeltaSeconds :type Float%20%28single-precision%29))
  (bind _digprogress (Variables|Default|GetDigProgress))
  (bind _interactingcamera (Variables|Default|GetInteractingCamera))
  (CallFunction|SetGraveResourceAvailableText)
  (Utilities|IsValid _interactingcamera
    (:Is%20Valid
      (Transformation|SetWorldRotation _digprogress (Math|Rotator|FindLookatRotation (Transformation|GetWorldLocation _digprogress) (Transformation|GetWorldLocation _interactingcamera)) false false))))

(fn ConstructionScript)

(fn SetGraveType
  (params (GraveType :type EResourceGenerate%20Enum :default "NewEnumerator2"))
  (bind _output_get (Variables|Default|SetGraveType GraveType))
  (switch Utilities|FlowControl|Switch|SwitchonEResourceGenerate _output_get
    (:NewEnumerator4
      (bind _returnvalue (AddComponent|AddAIPerceptionStimuliSourceComponent))
      (bind _output_get_2 (Variables|Default|SetCrystalStimulus _returnvalue))
      (Class|AIPerceptionStimuliSourceComponent|RegisterforSense _output_get_2 "/Script/AIModule.AISense_Hearing")
      (Class|AIPerceptionStimuliSourceComponent|RegisterwithPerceptionSystem _output_get_2)
      (Utilities|Time|SetTimerbyFunctionName 0 "PingCrystalGraveStimulus" (Variables|Default|GetCrystalPing) true))))

(fn PingCrystalGraveStimulus
  (Class|AISenseHearing|ReportNoiseEvent (Transformation|GetActorLocation) 1.0 self 0.0 "Crystal"))

(fn SetGraveResourceAvailableText
  (if (not (Variables|Default|GetbResourcesAvailable))
    (Rendering|Components|TextRender|SetText (Variables|Default|GetTimerText) (Utilities|Text|FormatText "{RemainingTime}" (Utilities|Time|GetTimerRemainingTimebyHandle (Variables|Default|GetRechargeTimer))))))