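; BP_Pit is an interactable pit that collects essence and spawns a boss once enough has been gathered.
; AddEssenceToPit adds the given amount to a running total and calls ConsumeStoredEssence when the total reaches the threshold.
; ConsumeStoredEssence resets the total to zero, discarding any excess, and spawns the configured boss class at the pit's transform.
; The event graph and construction script hold no logic.
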(event EventBeginPlay)

(event Collision|EventActorBeginOverlap
  (params (OtherActor :type Actor%20Object%20Reference)))

(event EventTick
  (params (DeltaSeconds :type Float%20%28single-precision%29)))

(fn ConstructionScript)

(fn AddEssencetoPit
  (params (Amount :type Float%20%28double-precision%29))
  (bind _output_get (Variables|Default|SetEssenceCollected (+ Amount (Variables|Default|GetEssenceCollected))))
  (if (>= _output_get (Variables|Default|GetEssenceThreshold))
    (CallFunction|ConsumeStoredEssence)
    (else
      (return))))

(fn ConsumeStoredEssence
  (Variables|Default|SetEssenceCollected 0.0)
  (Game|SpawnActorfromClass (Variables|Default|GetPitBossClass) (Transformation|GetActorTransform) "Undefined" "MultiplyWithRoot" 0 0))